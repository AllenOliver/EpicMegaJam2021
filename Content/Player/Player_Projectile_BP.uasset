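; Player projectile that takes on the red or blue color of the player's current Shift state.
; On BeginPlay it plays a sound, sets its sphere material and point light to that color, and launches at max speed along the negated forward vector of the player's MouseDirection yaw.
; OnDestroy waits briefly, spawns the color-matched explosion, plays a sound and destroys the actor; nothing in this graph calls it, and the collision overlap is empty.
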(event OnComponentBeginOverlap(Collision)
  (params (OverlappedComponent :type Primitive%20Component%20Object%20Reference) (OtherActor :type Actor%20Object%20Reference) (OtherComp :type Primitive%20Component%20Object%20Reference) (OtherBodyIndex :type Integer) (bFromSweep :type Boolean) (SweepResult :type Hit%20Result%20Structure%20%28by%20ref%29)))

(event EventBeginPlay
  (bind _sphere (Variables|Default|GetSphere))
  (bind _projectilemovement (Variables|Default|GetProjectileMovement))
  (bind _pointlight (Variables|Default|GetPointLight))
  (Audio|PlaySoundatLocation "/Game/Sounds/E.E" (Transformation|GetWorldLocation (Variables|Default|GetSphere)) "0, 0, 0" 1.0 1.0 0.0 0 0 0)
  (bind _asplayer_pawn (Utilities|Casting|CastToPlayerPawn (Game|GetPlayerCharacter 0)))
  (bind _returnvalue (Class|ACShift|GetCurrentColor (Variables|/Script/EMJ_2021.EMJ_2021Character|GetShift _asplayer_pawn)))
  (Variables|Default|SetCurrent_Color _returnvalue)
  (if (Utilities|Enum|Equal(Enum) (Variables|Default|GetCurrent_Color) "RED")
    (Rendering|Material|SetMaterial _sphere 0 "/Game/Materials/M_Red_Emissive.M_Red_Emissive")
    (Rendering|Components|Light|SetLightColor _pointlight (Math|Conversions|ToLinearColor(Color) (Variables|Default|GetRed_Light)) true)
    (else
      (Rendering|Material|SetMaterial _sphere 0 "/Game/Materials/M_Blue_Emissive.M_Blue_Emissive")
      (Rendering|Components|Light|SetLightColor _pointlight (Math|Conversions|ToLinearColor(Color) (Variables|Default|GetBlue_Light)) true)))
  (Variables|/Script/Engine.MovementComponent|SetVelocity _projectilemovement (* (* (Class|MovementComponent|GetMaxSpeed _projectilemovement) (Math|Vector|GetForwardVector (Math|Rotator|MakeRotator 0.0 0.0 (Variables|/Game/Player/PlayerPawn.PlayerPawn_C|GetMouse_Direction _asplayer_pawn)))) -1.0)))

(event Collision|EventActorBeginOverlap
  (params (OtherActor :type Actor%20Object%20Reference)))

(event EventTick
  (params (DeltaSeconds :type Float%20%28single-precision%29)))

(event EventOnDestroy
  (bind _sphere (Variables|Default|GetSphere))
  (bind _returnvalue (Transformation|GetWorldTransform _sphere))
  (Utilities|FlowControl|Delay 0.015)
  (if (Utilities|Enum|Equal(Enum) (Variables|Default|GetCurrent_Color) "RED")
    (Game|SpawnActorfromClass "/Game/Red_Explosion_BP.Red_Explosion_BP_C" _returnvalue "Undefined" 0 0)
    (else
      (Game|SpawnActorfromClass "/Game/Blue_Explosion_BP.Blue_Explosion_BP_C" _returnvalue "Undefined" 0 0)))
  (Audio|PlaySoundatLocation "/Game/Sounds/A.A" (Transformation|GetWorldLocation (Variables|Default|GetSphere)) "0, 0, 0" 1.0 1.0 0.0 0 0 0)
  (Actor|DestroyActor))

(fn ConstructionScript)