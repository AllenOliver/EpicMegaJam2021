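; Player projectile Blueprint that flies along the player's aim and explodes on overlap.
; On BeginPlay it casts player 0 to MyEMJ_2021Character and sets velocity to max speed along the negated forward vector of the MouseDirection yaw.
; Any Collision overlap spawns a red or blue explosion at the Sphere transform according to GetColor, then destroys the projectile.
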(event OnComponentBeginOverlap(Collision)
  (params (OverlappedComponent :type Primitive%20Component%20Object%20Reference) (OtherActor :type Actor%20Object%20Reference) (OtherComp :type Primitive%20Component%20Object%20Reference) (OtherBodyIndex :type Integer) (bFromSweep :type Boolean) (SweepResult :type Hit%20Result%20Structure%20%28by%20ref%29))
  (bind _sphere (Variables|Default|GetSphere))
  (bind _returnvalue (Transformation|GetWorldTransform _sphere))
  (bind _returnvalue_2 (Class|PlayerProjectile|GetColor))
  (if (Utilities|Enum|Equal(Enum) _returnvalue_2 "RED")
    (Game|SpawnActorfromClass "/Game/Red_Explosion_BP.Red_Explosion_BP_C" _returnvalue "Undefined" 0 0)
    (else
      (Game|SpawnActorfromClass "/Game/Blue_Explosion_BP.Blue_Explosion_BP_C" _returnvalue "Undefined" 0 0)))
  (Actor|DestroyActor))

(event EventBeginPlay
  (bind _projectilemovement (Variables|Default|GetProjectileMovement))
  (bind _asmy_emj_2021character (Utilities|Casting|CastToMyEMJ_2021Character (Game|GetPlayerCharacter 0)))
  (Variables|/Script/Engine.MovementComponent|SetVelocity _projectilemovement (* (* (Class|MovementComponent|GetMaxSpeed _projectilemovement) (Math|Vector|GetForwardVector (Math|Rotator|MakeRotator 0.0 0.0 (Variables|/Game/MyEMJ_2021Character.MyEMJ_2021Character_C|GetMouse_Direction _asmy_emj_2021character)))) -1.0)))

(event Collision|EventActorBeginOverlap
  (params (OtherActor :type Actor%20Object%20Reference)))

(event EventTick
  (params (DeltaSeconds :type Float%20%28single-precision%29)))

(fn ConstructionScript)