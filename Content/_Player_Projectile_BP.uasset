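; Player projectile Actor that takes on the player's current shift color, red or blue, when it spawns.
; BeginPlay reads that color to set the sphere material and point light, then launches along the reverse of the player's MouseDirection yaw at the projectile movement's max speed.
; Its OnDestroy event spawns the color-matched explosion at the sphere's transform, destroys the actor and sets a hit flag.
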(event EventBeginPlay
  (bind _sphere (Variables|Default|GetSphere))
  (bind _projectilemovement (Variables|Default|GetProjectileMovement))
  (bind _pointlight (Variables|Default|GetPointLight))
  (bind _asmy_emj_2021character (Utilities|Casting|CastToMyEMJ_2021Character (Game|GetPlayerCharacter 0)))
  (bind _returnvalue (Class|ACShift|GetCurrentColor (Variables|/Script/EMJ_2021.EMJ_2021Character|GetShift _asmy_emj_2021character)))
  (Variables|Default|SetCurrent_Color _returnvalue)
  (if (Utilities|Enum|Equal(Enum) (Variables|Default|GetCurrent_Color) "RED")
    (Rendering|Material|SetMaterial _sphere 0 "/Game/Materials/M_Red_Emissive.M_Red_Emissive")
    (Rendering|Components|Light|SetLightColor _pointlight (Math|Conversions|ToLinearColor(Color) (Variables|Default|GetRed_Light)) true)
    (else
      (Rendering|Material|SetMaterial _sphere 0 "/Game/Materials/M_Blue_Emissive.M_Blue_Emissive")
      (Rendering|Components|Light|SetLightColor _pointlight (Math|Conversions|ToLinearColor(Color) (Variables|Default|GetBlue_Light)) true)))
  (Variables|/Script/Engine.MovementComponent|SetVelocity _projectilemovement (* (* (Class|MovementComponent|GetMaxSpeed _projectilemovement) (Math|Vector|GetForwardVector (Math|Rotator|MakeRotator 0.0 0.0 (Variables|/Game/MyEMJ_2021Character.MyEMJ_2021Character_C|GetMouse_Direction _asmy_emj_2021character)))) -1.0)))

(event Collision|EventActorBeginOverlap
  (params (OtherActor :type Actor%20Object%20Reference)))

(event EventTick
  (params (DeltaSeconds :type Float%20%28single-precision%29)))

(event EventOnDestroy
  (bind _sphere (Variables|Default|GetSphere))
  (bind _returnvalue (Transformation|GetWorldTransform _sphere))
  (if (Utilities|Enum|Equal(Enum) (Variables|Default|GetCurrent_Color) "RED")
    (Game|SpawnActorfromClass "/Game/Red_Explosion_BP.Red_Explosion_BP_C" _returnvalue "Undefined" 0 0)
    (else
      (Game|SpawnActorfromClass "/Game/Blue_Explosion_BP.Blue_Explosion_BP_C" _returnvalue "Undefined" 0 0)))
  (Actor|DestroyActor)
  (Variables|Default|SetHasHit_0 true))

(fn ConstructionScript)